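; BP_Simulation is a Blueprint that sets up and starts a simulation inside a cell when play begins.
; BeginPlay creates the cell with a width and color, sets the temperature from Celsius converted to Kelvin, then calls InitializeSimulation.
; It also queries volume, converted to liters, plus temperature and energy without using the results; the simulation functions are defined outside this graph.
; Unconnected cell-resizing nodes never run.
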(event EventBeginPlay
  (Class|Simulation|InitSimulationCell 1e+03 (Math|Color|MakeColor 255 255 0 255))
  (bind _returnvalue (Class|Simulation|ConvertCtoK 32.0))
  (Class|Simulation|SetSimulationTemp _returnvalue)
  (bind _returnvalue_2 (Class|Simulation|GetSimulationVolume))
  (Class|Simulation|ConvertPm3toL _returnvalue_2)
  (Class|Simulation|GetSimulationTemp)
  (Class|Simulation|GetSimulationEnergy)
  (Class|Simulation|InitializeSimulation))

(event Collision|EventActorBeginOverlap
  (params (OtherActor :type Actor%20Object%20Reference)))

(event EventTick
  (params (DeltaSeconds :type Float%20%28single-precision%29)))

(fn ConstructionScript)